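; Actor component for a player pawn that previews an adjustable card-throw trajectory and spawns BP_Card toward the mouse hit point.
; At BeginPlay it creates a two-point spline and cylinder spline mesh on the owner, then each Tick follows the owner and cursor hit.
; Holding the trajectory input freezes the endpoint while mouse movement bends the tangents, then restores the cursor on release.
; A separate height input adjusts the tangents' Z to arc the curve.
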(event `self.ReceiveBeginPlay`
  (`self.CreateSpline`)
  (`self.CreateSplineMesh`))

(event `self.ReceiveTick`
  (params (DeltaSeconds :type "Float (single-precision)"))
  (`self.UpdateSplinesLocations`)
  (`self.UpdateSplineMesh`))

(event `EnhancedInput|/Game/Casino/Input/Actions/Cards/IA_ChangeTrajectory`
  (params (ActionValue :type Boolean) (ElapsedSeconds :type "Float (double-precision)") (TriggeredSeconds :type "Float (double-precision)") (InputAction :type "InputAction Object Reference" :default "/Game/Casino/Input/Actions/Cards/IA_ChangeTrajectory.IA_ChangeTrajectory"))
  (:`Triggered`
    (`self.ChangeTrajectory`))
  (:`Started`
    (`self.StartChangingTrajectory`))
  (:`Canceled`
    (`self.StopChangingTrajectory` :!label _label))
  (:`Completed`
    (goto _label)))

(event `EnhancedInput|/Game/Casino/Input/Actions/Cards/IA_ChangeTrajectoryHeight`
  (params (ActionValue :type "Float (double-precision)") (ElapsedSeconds :type "Float (double-precision)") (TriggeredSeconds :type "Float (double-precision)") (InputAction :type "InputAction Object Reference" :default "/Game/Casino/Input/Actions/Cards/IA_ChangeTrajectoryHeight.IA_ChangeTrajectoryHeight"))
  (:`Triggered`
    (`self.ChangeTrajectoryHeight` ActionValue)))

(event `EnhancedInput|/Game/Casino/Input/Actions/Cards/IA_ThrowCard`
  (params (ActionValue :type Boolean) (ElapsedSeconds :type "Float (double-precision)") (TriggeredSeconds :type "Float (double-precision)") (InputAction :type "InputAction Object Reference" :default "/Game/Casino/Input/Actions/Cards/IA_ThrowCard.IA_ThrowCard"))
  (:`Triggered`
    (`self.ThrowCard`)))

(fn `ChangeTrajectory`
  (bind _trajectorychangesensitivity (`self.TrajectoryChangeSensitivity`))
  (bind (_returnvalue_x _returnvalue_y _returnvalue_z) (`KismetMathLibrary.BreakVector` (`SplineComponent.GetTangentAtSplinePoint` (`self.Spline`) 0 "World")))
  (bind (_returnvalue_x_2 _returnvalue_y_2 _returnvalue_z_2) (`KismetMathLibrary.BreakVector` (`SplineComponent.GetTangentAtSplinePoint` (`self.Spline`) 1 "World")))
  (bind _aspawn (cast `Pawn` (`self.GetOwner`)))
  (bind _asbp_player_controller (cast `/Game/Casino/Blueprints/Player/BP_PlayerController` (`Pawn.GetController` _aspawn)))
  (bind (_returnvalue_x_3 _returnvalue_y_3) (`KismetMathLibrary.BreakVector` (- (`/Game/Casino/Blueprints/Player/BP_PlayerController.GetMouseWorldLocation` _asbp_player_controller) (`self.StartMouseLocation`))))
  (`SplineComponent.SetTangentAtSplinePoint` (`self.Spline`) 0 (`KismetMathLibrary.MakeVector` _returnvalue_x_3 _returnvalue_y_3 _returnvalue_z) "World" false)
  (`SplineComponent.SetTangentAtSplinePoint` (`self.Spline`) 1 (`KismetMathLibrary.MakeVector` (* _returnvalue_x_3 -1.0 _trajectorychangesensitivity) (* _returnvalue_y_3 -1.0 _trajectorychangesensitivity) _returnvalue_z_2) "World" false)
  (`SplineComponent.SetLocationAtSplinePoint` (`self.Spline`) 1 (- (`self.StartSplineEndPosition`) (`Actor.K2_GetActorLocation` (`self.GetOwner`))) "Local" true))

(fn `ChangeTrajectoryHeight`
  (params (Value :type "Float (double-precision)"))
  (bind (_returnvalue_x _returnvalue_y _returnvalue_z) (`KismetMathLibrary.BreakVector` (`SplineComponent.GetTangentAtSplinePoint` (`self.Spline`) 1 "Local")))
  (bind (_returnvalue_x_2 _returnvalue_y_2 _returnvalue_z_2) (`KismetMathLibrary.BreakVector` (`SplineComponent.GetTangentAtSplinePoint` (`self.Spline`) 0 "Local")))
  (bind _returnvalue (* Value (`self.TrajectoryHeightChangeSensitivity`)))
  (`SplineComponent.SetTangentAtSplinePoint` (`self.Spline`) 1 (`KismetMathLibrary.MakeVector` _returnvalue_x _returnvalue_y (- _returnvalue_z _returnvalue)) "Local" false)
  (`SplineComponent.SetTangentAtSplinePoint` (`self.Spline`) 0 (`KismetMathLibrary.MakeVector` _returnvalue_x_2 _returnvalue_y_2 (+ _returnvalue_z_2 _returnvalue)) "Local" true))

(fn `CreateSpline`
  (bind _returnvalue (`|AddComponentByClass` :`self` (`self.GetOwner`) :`Class` "/Script/Engine.SplineComponent" :`bManualAttachment` true))
  (bind _output_get (set `self.Spline` _returnvalue))
  (`SceneComponent.SetMobility` _output_get "Movable")
  (`SceneComponent.K2_AttachToComponent` (`self.Spline`) (`Actor.RootComponent` (`self.GetOwner`)) "None" "KeepWorld" "KeepWorld" "KeepWorld" false)
  (set `SceneComponent.bAbsoluteLocation` true (`self.Spline`))
  (set `SceneComponent.bAbsoluteRotation` true (`self.Spline`)))

(fn `CreateSplineMesh`
  (bind _returnvalue (`|AddComponentByClass` :`self` (`self.GetOwner`) :`Class` "/Script/Engine.SplineMeshComponent" :`bManualAttachment` true))
  (bind _output_get (set `self.SplineMesh` _returnvalue))
  (`SceneComponent.SetMobility` _output_get "Movable")
  (`SceneComponent.K2_AttachToComponent` (`self.SplineMesh`) (`Actor.RootComponent` (`self.GetOwner`)) "None" "KeepWorld" "KeepWorld" "KeepWorld" false)
  (set `SceneComponent.bAbsoluteLocation` true (`self.SplineMesh`))
  (set `SceneComponent.bAbsoluteRotation` true (`self.SplineMesh`))
  (`StaticMeshComponent.SetStaticMesh` (`self.SplineMesh`) "/Engine/BasicShapes/Cylinder.Cylinder")
  (`PrimitiveComponent.SetMaterial` (`self.SplineMesh`) 0 "/Game/Casino/Materials/M_Spline.M_Spline")
  (`SplineMeshComponent.SetForwardAxis` (`self.SplineMesh`) "Z" true)
  (`SplineMeshComponent.SetStartScale` (`self.SplineMesh`) (0.05 0.05) true)
  (`SplineMeshComponent.SetEndScale` (`self.SplineMesh`) (0.05 0.05) true))

(fn `ResetSpline`
  (`SplineMeshComponent.SetEndTangent` (`self.SplineMesh`) (0.0 0.0 0.0) true)
  (`SplineComponent.SetTangentAtSplinePoint` (`self.Spline`) 1 (0.0 0.0 0.0) "Local" true)
  (`SplineMeshComponent.SetStartTangent` (`self.SplineMesh`) (0.0 0.0 0.0) true)
  (`SplineComponent.SetTangentAtSplinePoint` (`self.Spline`) 0 (0.0 0.0 0.0) "Local" true))

(fn `StartChangingTrajectory`
  (`self.ResetSpline`)
  (set `self.UpdateEndPosition` false)
  (bind _aspawn (cast `Pawn` (`self.GetOwner`)))
  (bind _asbp_player_controller (cast `/Game/Casino/Blueprints/Player/BP_PlayerController` (`Pawn.GetController` _aspawn)))
  (set `self.StartMouseLocation` (`/Game/Casino/Blueprints/Player/BP_PlayerController.GetMouseWorldLocation` _asbp_player_controller))
  (set `self.StartSplineEndPosition` (+ (`SplineMeshComponent.GetEndPosition` (`self.SplineMesh`)) (`Actor.K2_GetActorLocation` (`self.GetOwner`)))))

(fn `StopChangingTrajectory`
  (set `self.UpdateEndPosition` true)
  (bind _aspawn (cast `Pawn` (`self.GetOwner`)))
  (bind _asbp_player_controller (cast `/Game/Casino/Blueprints/Player/BP_PlayerController` (`Pawn.GetController` _aspawn)))
  (bind (_x _y) (`KismetMathLibrary.BreakVector2D` (`GameplayStatics.ProjectWorldToScreen` _asbp_player_controller (`self.StartMouseLocation`) true)))
  (`PlayerController.SetMouseLocation` _asbp_player_controller (`KismetMathLibrary.FTrunc` _x) (`KismetMathLibrary.FTrunc` _y)))

(fn `ThrowCard`
  (bind _aspawn (cast `Pawn` (`self.GetOwner`)))
  (bind _asbp_player_controller (cast `/Game/Casino/Blueprints/Player/BP_PlayerController` (`Pawn.GetController` _aspawn)))
  (bind _aspawn_2 (cast `Pawn` (`self.GetOwner`)))
  (`|SpawnActorFromClass` "/Game/Casino/Blueprints/Cards/BP_Card.BP_Card_C" (`KismetMathLibrary.MakeTransform` (`SceneComponent.K2_GetComponentLocation` (`Actor.GetComponentByClass` (`self.GetOwner`) "/Script/Engine.SplineComponent")) (`KismetMathLibrary.FindLookAtRotation` (`Actor.K2_GetActorLocation` (`self.GetOwner`)) (`/Game/Casino/Blueprints/Player/BP_PlayerController.GetMouseWorldLocationByHit` _asbp_player_controller))) "Undefined" "MultiplyWithRoot" (`self.GetOwner`) _aspawn_2))

(fn `UpdateSplineMesh`
  (bind (_location _tangent) (`SplineComponent.GetLocationAndTangentAtSplinePoint` (`self.Spline`) 1 "Local"))
  (bind (_location_2 _tangent_2) (`SplineComponent.GetLocationAndTangentAtSplinePoint` (`self.Spline`) 0 "Local"))
  (`SplineMeshComponent.SetStartAndEnd` (`self.SplineMesh`) _location_2 _tangent_2 _location _tangent true))

(fn `UpdateSplinesLocations`
  (`SceneComponent.K2_SetWorldLocation` (`self.SplineMesh`) (`Actor.K2_GetActorLocation` (`self.GetOwner`)) false false)
  (`SceneComponent.K2_SetWorldLocation` (`self.Spline`) (`Actor.K2_GetActorLocation` (`self.GetOwner`)) false false)
  (if (`self.UpdateEndPosition`)
    (bind _aspawn (cast `Pawn` (`self.GetOwner`)))
    (bind _asbp_player_controller (cast `/Game/Casino/Blueprints/Player/BP_PlayerController` (`Pawn.GetController` _aspawn)))
    (`SplineComponent.SetLocationAtSplinePoint` (`self.Spline`) 1 (`/Game/Casino/Blueprints/Player/BP_PlayerController.GetMouseWorldLocationByHit` _asbp_player_controller) "World" true)))