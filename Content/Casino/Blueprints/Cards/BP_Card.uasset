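; Spinning card projectile that flies along a curved path and damages what it strikes through the Gameplay Ability System.
; BeginPlay randomizes spin and copies the owner's two-point spline, which Tick follows, then continues along the end tangent.
; Hits and non-owner overlaps apply a damage effect to ability-system targets; such hits also freeze the card and strip its components.
; The spawn-on-hit and ApplyDamage fallback logic is unwired.
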(event `self.ReceiveBeginPlay`
  (`self.SetRandomRotationRate`)
  (`self.CopySplineFromOwner`))

(event `self.ReceiveTick`
  (params (DeltaSeconds :type "Float (single-precision)"))
  (`self.Update Card Velocity`)
  (`self.UpdateCardRotation`))

(event `self.Box.OnComponentHit`
  (params (HitComponent :type "PrimitiveComponent Object Reference") (OtherActor :type "Actor Object Reference") (OtherComp :type "PrimitiveComponent Object Reference") (NormalImpulse :type "Vector Structure") (Hit :type "HitResult Structure (by ref)"))
  (bind _returnvalue (`AbilitySystemBlueprintLibrary.GetAbilitySystemComponent` OtherActor))
  (`/Engine/EditorBlueprintResources/StandardMacros.IsValid` _returnvalue
    (:`Is Valid`
      (`AbilitySystemComponent.BP_ApplyGameplayEffectToSelf` _returnvalue "/Game/Casino/Blueprints/AbilitySystem/GameplayEffects/BP_DamageGameplayEffect.BP_DamageGameplayEffect_C" 0.0 (`AbilitySystemComponent.MakeEffectContext` _returnvalue))
      (`self.SetActorTickEnabled` false)
      (bind _box (`self.Box`)
        (:`then`
          (`ActorComponent.K2_DestroyComponent` _box))
        (:`else`
          _))
      (bind _rotatingmovement (`self.RotatingMovement`)
        (:`then`
          (`ActorComponent.K2_DestroyComponent` _rotatingmovement))
        (:`else`
          _))
      (bind _spline (`self.Spline`)
        (:`then`
          (`ActorComponent.K2_DestroyComponent` _spline))
        (:`else`)))))

(event `self.Box.OnComponentBeginOverlap`
  (params (OverlappedComponent :type "PrimitiveComponent Object Reference") (OtherActor :type "Actor Object Reference") (OtherComp :type "PrimitiveComponent Object Reference") (OtherBodyIndex :type Integer) (bFromSweep :type Boolean) (SweepResult :type "HitResult Structure (by ref)"))
  (bind _returnvalue (`AbilitySystemBlueprintLibrary.GetAbilitySystemComponent` OtherActor))
  (if (!= OtherActor (`self.GetOwner`))
    (`/Engine/EditorBlueprintResources/StandardMacros.IsValid` _returnvalue
      (:`Is Valid`
        (`AbilitySystemComponent.BP_ApplyGameplayEffectToSelf` _returnvalue "/Game/Casino/Blueprints/AbilitySystem/GameplayEffects/BP_DamageGameplayEffect.BP_DamageGameplayEffect_C" 0.0 (`AbilitySystemComponent.MakeEffectContext` _returnvalue))))))

(fn `CopySplineFromOwner`
  (bind _returnvalue (`self.GetComponentByClass` (`self.GetOwner`) "/Script/Engine.SplineComponent"))
  (bind _returnvalue_2 (`AddComponent|NODE_AddSplineComponent-0`))
  (bind _output_get (set `self.Spline` _returnvalue_2))
  (set `SceneComponent.bAbsoluteLocation` true (`self.Spline`))
  (set `SceneComponent.bAbsoluteRotation` true (`self.Spline`))
  (`SceneComponent.K2_SetWorldLocation` _output_get (`self.K2_GetActorLocation` (`self.GetOwner`)) false false)
  (`SceneComponent.K2_SetWorldLocation` (`self.Spline`) (`self.K2_GetActorLocation` (`self.GetOwner`)) false false)
  (`SplineComponent.ClearSplinePoints` (`self.Spline`) false)
  (`SplineComponent.AddPoint` (`self.Spline`) (`SplineComponent.GetSplinePointAt` _returnvalue 0 "Local") false)
  (`SplineComponent.AddPoint` (`self.Spline`) (`SplineComponent.GetSplinePointAt` _returnvalue 1 "Local") true))

(fn `SetRandomRotationRate`
  (set `RotatingMovementComponent.RotationRate` (`KismetMathLibrary.MakeRotator` 0.0 0.0 (`KismetMathLibrary.RandomFloatInRange` 1000.0 2000.0)) (`self.RotatingMovement`)))

(fn `SpawnActors`
  (returns (SpawnedAtLeastOne :type Boolean))
  (locals (SpawnedAtLeastOnce :type Boolean))
  (for _array_element (`self.ActorsToSpawnOnHit`)
    (if (`KismetSystemLibrary.IsValidSoftClassReference` _array_element)
      (bind _returnvalue (`KismetSystemLibrary.LoadClassAsset_Blocking` _array_element))
      (bind _asactor (castclass `Actor` _returnvalue))
      (`|SpawnActorFromClass` _asactor (`self.GetTransform`) "AdjustIfPossibleButAlwaysSpawn" "MultiplyWithRoot" self (`self.Instigator`))
      (set `local.SpawnedAtLeastOnce` true)))
  (return (`local.SpawnedAtLeastOnce`)))

(fn `Update Card Velocity`
  (locals (PreviousLocation :type "Vector Structure" :default (0.0 0.0 0.0)))
  (bind _returnvalue (+ (* (`KismetMathLibrary.Normal` (`SplineComponent.FindTangentClosestToWorldLocation` (`self.Spline`) (`self.K2_GetActorLocation`) "World")) (`self.CardSpeed`)) (`self.K2_GetActorLocation`)))
  (bind _returnvalue_2 (`SplineComponent.FindLocationClosestToWorldLocation` (`self.Spline`) _returnvalue "World"))
  (bind _output_get (set `local.PreviousLocation` (`self.K2_GetActorLocation`)))
  (if (or (`self.ReachedFinalSplinePoint`) (== _output_get (`SplineComponent.GetLocationAtSplinePoint` (`self.Spline`) 1 "World") :`ErrorTolerance` 0.1))
    (set `self.ReachedFinalSplinePoint` true)
    ;[1 1 1] Move along last tangent
    (`self.K2_SetActorLocation` (+ (* (`KismetMathLibrary.Normal` (`SplineComponent.GetTangentAtSplinePoint` (`self.Spline`) 1 "World")) (`self.CardSpeed`)) (`self.K2_GetActorLocation`)) true)
    (elif (== _returnvalue_2 (`local.PreviousLocation`) :`ErrorTolerance` 0.1)
      (`self.K2_SetActorLocation` _returnvalue true)
      (else
        (`self.K2_SetActorLocation` _returnvalue_2 true)))))

(fn `UpdateCardRotation`
  (bind _spline (`self.Spline`)
    (:`then`
      (`self.K2_SetActorRotation` (`KismetMathLibrary.Conv_VectorToRotator` (`SplineComponent.FindTangentClosestToWorldLocation` _spline (`self.K2_GetActorLocation`) "World"))))
    (:`else`)))

(fn `UserConstructionScript`)