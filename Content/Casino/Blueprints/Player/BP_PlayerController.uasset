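; Player controller for the Casino game that shows the mouse cursor on BeginPlay and offers two helpers for finding the cursor's world position.
; GetMouseWorldLocationByHit returns the hit location of a complex trace under the cursor on the Camera channel.
; GetMouseWorldLocation deprojects the mouse and intersects that ray with the Z=0 plane mathematically, so it needs no collision.
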(event `self.ReceiveBeginPlay`
  (set `self.bShowMouseCursor` true))

(fn `GetMouseWorldLocation`
  (returns (Location :type "Vector Structure"))
  (bind (_worldlocation _worlddirection) (`self.DeprojectMousePositionToWorld`))
  (return (+ _worldlocation (* (/ (.z _worldlocation) (.z _worlddirection)) -1.0 _worlddirection))))

(fn `GetMouseWorldLocationByHit`
  (returns (Location :type "Vector Structure"))
  (return (`.Location` (`GameplayStatics.BreakHitResult` (`self.GetHitResultUnderCursorByChannel` "TraceTypeQuery2")))))

(fn `UserConstructionScript`)