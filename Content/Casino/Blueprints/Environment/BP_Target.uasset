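; A casino target that a thrown BP_Card slices in two on impact.
; The construction script copies the static TargetMesh into a procedural mesh with collision so it can be cut at runtime.
; A card hit plays a bell, slices the mesh at the impact point along the card's up vector without caps, and sets both halves simulating physics.
; The card is destroyed, and its owning player gets a faint white camera flash.
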(event `self.ProceduralMesh.OnComponentHit`
  (params (HitComponent :type "PrimitiveComponent Object Reference") (OtherActor :type "Actor Object Reference") (OtherComp :type "PrimitiveComponent Object Reference") (NormalImpulse :type "Vector Structure") (Hit :type "HitResult Structure (by ref)"))
  (cast `/Game/Casino/Blueprints/Cards/BP_Card` OtherActor)
  (`GameplayStatics.PlaySound2D` "/Game/Casino/Sound/SW_Bell.SW_Bell" 1.0 1.0 0.0 null null)
  (`PrimitiveComponent.SetSimulatePhysics` (`self.ProceduralMesh`) true)
  (bind _outotherhalfprocmesh (`KismetProceduralMeshLibrary.SliceProceduralMesh` (`self.ProceduralMesh`) (`.Location` (`GameplayStatics.BreakHitResult` Hit)) (`self.GetActorUpVector` OtherActor) true "NoCap"))
  (`PrimitiveComponent.SetSimulatePhysics` _outotherhalfprocmesh true)
  (bind _aspawn (cast `Pawn` (`self.GetOwner` OtherActor))
    (:`then`
      (bind _asplayer_controller (cast `PlayerController` (`Pawn.GetController` _aspawn))
        (:`then`
          (`PlayerCameraManager.StartCameraFade` (`PlayerController.PlayerCameraManager` _asplayer_controller) 0.05 0.0 1.0 (struct :`R` 1.0 :`G` 1.0 :`B` 1.0 :`A` 1.0) false false))
        (:`CastFailed`
          _)))
    (:`CastFailed`
      _))
  (`self.K2_DestroyActor` OtherActor))

(fn `UserConstructionScript`
  (`KismetProceduralMeshLibrary.CopyProceduralMeshFromStaticMeshComponent` (`self.TargetMesh`) 0 (`self.ProceduralMesh`) true))